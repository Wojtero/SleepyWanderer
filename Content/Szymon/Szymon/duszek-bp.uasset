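; Duszek Blueprint is an actor that follows the mouse cursor in the world.
; Every Tick it deprojects player 0's mouse position into a world ray and teleports itself, without sweeping, to where that ray meets the Y=0 plane.
; The intersection comes from scaling the ray direction by the negated ratio of origin Y to direction Y, with no guard against a zero divisor.
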(event `self.ReceiveTick`
  (params (DeltaSeconds :type "Float (single-precision)"))
  (bind (_worldlocation _worlddirection) (`PlayerController.DeprojectMousePositionToWorld` (`GameplayStatics.GetPlayerController` 0)))
  (`self.K2_SetActorLocation` (+ _worldlocation (* (* _worlddirection (/ (`.Y` (`KismetMathLibrary.BreakVector2D` (`KismetMathLibrary.Conv_VectorToVector2D` _worldlocation))) (`.Y` (`KismetMathLibrary.BreakVector2D` (`KismetMathLibrary.Conv_VectorToVector2D` _worlddirection))))) -1.0)) false true))

(fn `UserConstructionScript`)